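; Lock-on camera mode that keeps the player's view turned toward the actor targeted by the owning character's TargetingComponent.
; Each tick it lerps control rotation toward a look-at from a point raised above the camera, clamping pitch and keeping roll.
; The lerp is stronger for nearby targets and uses a fixed alpha, independent of delta time.
; It falls back to BP_CameraModeBase when the controller or target is invalid.
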(event EventStartCameraMode
  (bind _ascharacter (Utilities|Casting|CastToCharacter (Components|GetOwner (Variables|Default|GetCameraModeComponent))))
  (Variables|Default|SetLocal%20Player%20Controller (Pawn|GetController _ascharacter))
  (Variables|Default|SetLocal%20Targeting%20Component (Actor|GetComponentbyClass (Components|GetOwner (Variables|Default|GetCameraModeComponent)) "/Script/Outline.TargetingComponent"))
  (Class|CameraModeBase|SetCameraModeStatus "(TagName=\"Camera.Mode.Status.Looping\")"))

(event EventTickCameraMode
  (params (TickValue :type Float%20%28single-precision%29))
  (bind _local_targeting_component (Variables|Default|GetLocal%20Targeting%20Component))
  (bind _local_player_controller (Variables|Default|GetLocal%20Player%20Controller))
  (bind _returnvalue (Pawn|GetControlRotation _local_player_controller :!class /Script/Engine.Controller))
  (bind _returnvalue_2 (Class|TargetingComponent|GetTargetedActor _local_targeting_component))
  (Utilities|IsValid (Variables|Default|GetLocal%20Player%20Controller)
    (:Is%20Valid
      (Utilities|IsValid _returnvalue_2
        (:Is%20Valid
          (Variables|Default|SetTargeted%20Actor _returnvalue_2)
          (|SwitchGameplayTag (Variables|Default|GetCameraModeStatus)
            (:Camera.Mode.Status.Looping
              (Pawn|SetControlRotation (Variables|Default|GetLocal%20Player%20Controller) (Math|Rotator|MakeRotator (.Roll (Math|Rotator|BreakRotator _returnvalue)) (Math|Float|Clamp(Float) (.pitch (Math|Rotator|Lerp(Rotator) _returnvalue (Math|Rotator|FindLookatRotation (+ (Transformation|GetWorldLocation (Variables|/Script/Outline.CameraModeComponent|GetCameraComponent (Variables|Default|GetCameraModeComponent))) "0.000000,0.000000,100.000000") (Transformation|GetActorLocation (Variables|Default|GetTargeted%20Actor))) (select (< (Math|Vector|Distance(Vector) (Transformation|GetActorLocation (Variables|Default|GetTargeted%20Actor)) (Transformation|GetActorLocation (Components|GetOwner (Variables|Default|GetCameraModeComponent)))) 5e+02) 0.4 0.2) true)) -4e+01 3e+01) (.yaw (Math|Rotator|Lerp(Rotator) _returnvalue (Math|Rotator|FindLookatRotation (+ (Transformation|GetWorldLocation (Variables|/Script/Outline.CameraModeComponent|GetCameraComponent (Variables|Default|GetCameraModeComponent))) "0.000000,0.000000,100.000000") (Transformation|GetActorLocation (Variables|Default|GetTargeted%20Actor))) (select (< (Math|Vector|Distance(Vector) (Transformation|GetActorLocation (Variables|Default|GetTargeted%20Actor)) (Transformation|GetActorLocation (Components|GetOwner (Variables|Default|GetCameraModeComponent)))) 5e+02) 0.4 0.2) true)))))))
        (:Is%20Not%20Valid
          (Class|CameraModeComponent|SetCameraModeOfClass (Variables|Default|GetCameraModeComponent) "/Game/Blueprints/Camera/Mode/BP_CameraModeBase.BP_CameraModeBase_C" :!label _label))))
    (:Is%20Not%20Valid
      (goto _label))))