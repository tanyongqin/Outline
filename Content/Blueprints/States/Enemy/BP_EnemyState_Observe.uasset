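; Enemy AI state in which the enemy watches its combat target, then decides its next move after a short timer.
; Tick and the decision step rotate the enemy toward the target when it leaves the front yaw cone.
; The decision restarts on excessive distance or target death, switches to FollowTarget at mid range, or tries Attack up close, restarting on failure.
; Roll-away and random observe-ability logic exist but are unconnected.
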(event EventStartState
  (Utilities|Time|SetTimerbyFunctionName 0 "DecideNextState" 1.5))

(event EventDecideNextState
  (bind _returnvalue (Class|StateBase|GetStateManagerComponent))
  (bind _returnvalue_2 (Class|StateBase|GetStateManagerComponent))
  (bind _ownercharacter (Variables|Default|GetOwnerCharacter))
  (bind _combatcomponent (Variables|/Script/Outline.EnemyCharacterBase|GetCombatComponent _ownercharacter))
  (bind _returnvalue_3 (Class|EnemyStateBase|CalcYawandPitch))
  (if (Math|Float|InRange(Float) (.yaw _returnvalue_3) -45.0 45.0)
    (bind _returnvalue_4 (Class|EnemyCombatComponent|GetCombatTarget _combatcomponent))
    (bind _ascharacter_base (Utilities|Casting|CastToCharacterBase _returnvalue_4)
      (:then
        _)
      (:CastFailed
        _))
    (else
      (Class|EnemyCombatComponent|RotateEnemytoCombatTarget _combatcomponent 0.7)))
  (bind _returnvalue_5 (Class|EnemyStateBase|CalcDistance))
  (if (or (> _returnvalue_5 1.5e+03) (<= (Class|CharacterBase|GetCurrHealth _ascharacter_base) 0.0))
    (Class|StateBase|RestartState false) ; Can Replace With ReturnToPost
    (elif (> _returnvalue_5 8.5e+02)
      (Class|StateManagerComponent|PerformStateOfClass _returnvalue_2 (Utilities|GetClass (Class|StateManagerComponent|GetStateOfGameplayTag _returnvalue_2 "(TagName=\"State.FollowTarget\")")))
      (else
        (bind _returnvalue_6 (Class|StateManagerComponent|TryPerformStateOfClass _returnvalue (Utilities|GetClass (Class|StateManagerComponent|GetStateOfGameplayTag _returnvalue "(TagName=\"State.Attack\")")) true))
        (if (not _returnvalue_6)
          (Class|StateBase|RestartState false))))))

(event EventTickState
  (params (TickTime :type Float%20%28single-precision%29))
  ;[1 1 1] Rotate to target
  (bind _returnvalue (Class|EnemyStateBase|CalcYawandPitch))
  (if (not (Math|Float|InRange(Float) (.yaw _returnvalue) -45.0 45.0))
    (Class|EnemyCombatComponent|RotateEnemytoCombatTarget (Variables|/Script/Outline.EnemyCharacterBase|GetCombatComponent (Variables|Default|GetOwnerCharacter)) 0.1)))

(fn CanPerformState
  (return true))

(fn KeepAwayfromTarget
  (Class|AbilityManagerComponent|TryPerformAbilityOfClass (Variables|/Script/Outline.EnemyCharacterBase|GetAbilityManager (Variables|Default|GetOwnerCharacter)) "/Game/Blueprints/Abilities/Enemy/BP_GS_EnemyAbility_Roll.BP_GS_EnemyAbility_Roll_C" true)
  (Class|EnemyStateBase|DecideNextState))