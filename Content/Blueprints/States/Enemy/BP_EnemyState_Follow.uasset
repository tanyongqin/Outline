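; Enemy Follow state that sets walk speed by distance, presumably to the target, and hands off to Attack when close.
; Each tick it runs fast when far and drops to a walk when near, with a short timer delaying the slowdown.
; Close range triggers the next-state decision, where every random branch tries Attack (one rechecks distance first) and restarts Follow on failure.
; A random strafe transition exists but is unconnected.
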(event Custom|Reset%20Change%20In%20Speed
  (Variables|Default|SetChange%20in%20speed true))

(event EventTickState
  (params (TickTime :type Float%20%28single-precision%29))
  (CallFunction|AdjustMovementSpeedBasedonDistance)
  (bind _returnvalue (Class|EnemyStateBase|CalcDistance))
  (if (<= _returnvalue 3e+02)
    (Class|EnemyStateBase|DecideNextState)))

(event EventPrepareStateValues
  (CallFunction|AdjustMovementSpeedBasedonDistance))

(event EventDecideNextState
  (bind _returnvalue (Class|StateBase|GetStateManagerComponent))
  (|CallParentFunction)
  (switch int (Math|Random|RandomIntegerinRange 0 3)
    (:Default
      (bind _returnvalue_2 (Class|StateManagerComponent|TryPerformStateOfClass _returnvalue (Utilities|GetClass (Class|StateManagerComponent|GetStateOfGameplayTag _returnvalue "(TagName=\"State.Attack\")")) true :!label _label))
      (if (not _returnvalue_2)
        (Class|StateBase|RestartState false)))
    (:0
      (bind _returnvalue_3 (Class|EnemyStateBase|CalcDistance))
      (if (> _returnvalue_3 3e+02)
        (Class|StateBase|RestartState false)
        (else
          (goto _label))))
    (:1
      (goto _label))
    (:2
      (goto _label))))

(event EventStartState
  (Class|StateBase|StartStateTimer))

(fn CanPerformState
  (return true))

(fn AdjustMovementSpeedBasedonDistance
  (bind _returnvalue (Class|EnemyStateBase|CalcDistance))
  (if (>= _returnvalue 5e+02)
    (Variables|/Script/Engine.CharacterMovementComponent|SetMaxWalkSpeed (Variables|/Script/Engine.Character|GetCharacterMovement (Variables|Default|GetOwnerCharacter)) 7e+02)
    (Variables|Default|SetChange%20in%20speed false)
    (Utilities|Time|SetTimerbyFunctionName 0 "Reset Change In Speed" 1.5)
    (elif (and (< _returnvalue 5e+02) (Variables|Default|GetChange%20in%20speed))
      (Variables|/Script/Engine.CharacterMovementComponent|SetMaxWalkSpeed (Variables|/Script/Engine.Character|GetCharacterMovement (Variables|Default|GetOwnerCharacter)) 2.5e+02))))