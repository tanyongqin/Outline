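; Enemy turn state that performs a turn ability when a combat target exists and the calculated yaw is far enough off.
; It can run only if the absolute yaw exceeds a fixed threshold and the check on its TurnAbilities passes.
; On start, it performs the selected ability through the owner's AbilityManager.
; When deciding the next state, it calls the parent logic, then tries the FollowTarget state by gameplay tag with condition checking.
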(event EventStartState
  (Class|AbilityManagerComponent|PerformAbilityOfClass (Variables|/Script/Outline.EnemyCharacterBase|GetAbilityManager (Variables|Default|GetOwnerCharacter)) (Class|StateBase|GetSelectedAbility)))

(event EventDecideNextState
  (bind _returnvalue (Class|StateBase|GetStateManagerComponent))
  (|CallParentFunction)
  (Class|StateManagerComponent|TryPerformStateOfClass _returnvalue (Utilities|GetClass (Class|StateManagerComponent|GetStateOfGameplayTag _returnvalue "(TagName=\"State.FollowTarget\")")) true))

(fn CanPerformState
  (bind _returnvalue (Class|EnemyCombatComponent|GetCombatTarget (Variables|/Script/Outline.EnemyCharacterBase|GetCombatComponent (Variables|Default|GetOwnerCharacter))))
  (Utilities|IsValid _returnvalue
    (:Is%20Valid
      (bind _returnvalue_2 (Class|EnemyStateBase|CalcYawandPitch))
      (if (> (Math|Float|Absolute(Float) (.yaw _returnvalue_2)) 45.0)
        (bind _returnvalue_3 (Class|StateBase|CheckAbilitiestoRun (Variables|Default|GetTurn%20Abilities)))
        (return _returnvalue_3)
        (else
          (return false))))
    (:Is%20Not%20Valid
      (return false))))