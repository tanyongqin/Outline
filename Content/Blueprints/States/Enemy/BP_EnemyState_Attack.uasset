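; Enemy state that runs an attack ability on the owning character through its AbilityManager.
; It can be performed only when a valid combat target lacks the Death tag and the attack abilities pass their run check.
; On start it performs the selected ability, and when deciding the next state it switches to Observe, looked up by gameplay tag.
; Disconnected logic for restarting, turning or following the target never runs.
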(event EventDecideNextState
  (bind _returnvalue (Class|StateBase|GetStateManagerComponent))
  (|CallParentFunction)
  (Class|StateManagerComponent|PerformStateOfClass _returnvalue (Utilities|GetClass (Class|StateManagerComponent|GetStateOfGameplayTag _returnvalue "(TagName=\"State.Observe\")"))))

(event EventStartState
  (Class|AbilityManagerComponent|PerformAbilityOfClass (Variables|/Script/Outline.EnemyCharacterBase|GetAbilityManager (Variables|Default|GetOwnerCharacter)) (Class|StateBase|GetSelectedAbility)))

(fn CanPerformState
  (bind _returnvalue (Class|EnemyCombatComponent|GetCombatTarget (Variables|/Script/Outline.EnemyCharacterBase|GetCombatComponent (Variables|Default|GetOwnerCharacter))))
  (Utilities|IsValid _returnvalue
    (:Is%20Valid
      (bind _tagcontainer (GameplayTags|GetOwnedGameplayTags _returnvalue :!class /Script/GameplayTags.GameplayTagAssetInterface))
      (bind _returnvalue_2 (Class|StateBase|CheckAbilitiestoRun (Variables|Default|GetAttack%20Abilities)))
      (return (and _returnvalue_2 (not (GameplayTags|HasTag _tagcontainer "(TagName=\"State.Death\")")))))
    (:Is%20Not%20Valid
      (return false))))