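; Enemy death state that becomes available when health is at or below zero and the death ability check passes.
; On start it performs the selected ability and adds the State.Death tag if that ability class is valid.
; It always stops the AI brain logic, disables mesh and capsule collision and halts movement.
; DecideNextState is empty, so the state picks no successor.
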(event EventStartState
  (bind _returnvalue (Class|StateBase|GetSelectedAbility))
  (bind _ownercharacter (Variables|Default|GetOwnerCharacter))
  (bind _ownercharacter_2 (Variables|Default|GetOwnerCharacter))
  (bind _charactermovement (Variables|/Script/Engine.Character|GetCharacterMovement _ownercharacter))
  (|CallParentFunction)
  (if (Utilities|IsValidClass _returnvalue)
    (Class|AbilityManagerComponent|PerformAbilityOfClass (Variables|/Script/Outline.EnemyCharacterBase|GetAbilityManager (Variables|Default|GetOwnerCharacter)) _returnvalue)
    (GameplayTags|AddGameplayTag (Variables|/Script/Outline.CharacterBase|GetActorGameplayTags (Variables|Default|GetOwnerCharacter)) "(TagName=\"State.Death\")" :!class /Script/GameplayTags.BlueprintGameplayTagLibrary))
  (AI|Logic|StopLogic (Variables|/Script/AIModule.AIController|GetBrainComponent (AI|GetAIController (Variables|Default|GetOwnerCharacter))) "")
  (Collision|SetCollisionEnabled (Variables|/Script/Engine.Character|GetMesh _ownercharacter_2) "NoCollision")
  (Collision|SetCollisionEnabled (Variables|/Script/Engine.Character|GetCapsuleComponent _ownercharacter_2) "NoCollision")
  (Pawn|Components|CharacterMovement|DisableMovement _charactermovement)
  (Components|Movement|StopMovementImmediately _charactermovement))

(event EventEndState
  (|CallParentFunction)
  (Class|AbilityManagerComponent|PerformAbilityOfClass (Variables|/Script/Outline.EnemyCharacterBase|GetAbilityManager (Variables|Default|GetOwnerCharacter))))

(event EventDecideNextState)

(fn CanPerformState
  (bind _returnvalue (Class|StateBase|CheckAbilitiestoRun (Variables|Default|GetDeath%20Abilities)))
  (return (and _returnvalue (<= (Class|CharacterBase|GetCurrHealth (Variables|Default|GetOwnerCharacter)) 0.0))))