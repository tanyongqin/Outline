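; Enemy AI state for the equip phase, which in practice acts as a pass-through to the Observe state.
; Each tick it reads the combat target from the owner's CombatComponent and, if valid, asks the state manager to switch to the state tagged State.Observe, with condition checks.
; Start and prepare events are empty, and the equip ability call and debug print are disconnected, so no equipping happens here.
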(event EventTickState
  (params (TickTime :type Float%20%28single-precision%29))
  (bind _returnvalue (Class|EnemyCombatComponent|GetCombatTarget (Variables|/Script/Outline.EnemyCharacterBase|GetCombatComponent (Variables|Default|GetOwnerCharacter))))
  (Utilities|IsValid _returnvalue
    (:Is%20Valid
      (Class|EnemyStateBase|DecideNextState))))

(event EventStartState
  ;[1 1 1] //
)

(event EventPrepareStateValues)

(event EventDecideNextState
  (bind _returnvalue (Class|StateBase|GetStateManagerComponent))
  (Class|StateManagerComponent|TryPerformStateOfClass _returnvalue (Utilities|GetClass (Class|StateManagerComponent|GetStateOfGameplayTag _returnvalue "(TagName=\"State.Observe\")")) true))