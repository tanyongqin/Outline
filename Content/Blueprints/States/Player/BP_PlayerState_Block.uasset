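; Player block state for an ability-driven state machine, which slows walking and allows only movement and block inputs by default.
; It constructs missing block abilities, gates entry on the first one and performs the selected ability on start.
; Each tick polls the Block mapping's first key; release during Start ends the state, while release during Loop tries the End ability, ending the state on failure.
; Ending the state attempts a return to Idle.
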(event EventConstructState
  (bind _returnvalue (Class|PlayerStateBase|GetLocalAbilityManager))
  (|CallParentFunction)
  (bind _asplayer_controller (Utilities|Casting|CastToPlayerController (Pawn|GetController (Class|PlayerStateBase|GetOwnerCharacter))))
  (Variables|Default|SetOwner%20Player%20Controller _asplayer_controller)
  (for _array_element (Variables|Default|GetBlock%20Abilities)
    (Utilities|IsValid (Class|AbilityManagerComponent|GetAbilityOfClass _returnvalue _array_element)
      (:Is%20Not%20Valid
        (Class|AbilityManagerComponent|ConstructAbilityOfClass _returnvalue _array_element))))
  (Class|PlayerStateBase|ConstructDefaultAllowedInputs (Utilities|Array|MakeArray "MoveForward" "MoveRight" "Block")))

(event EventStartState
  (|CallParentFunction)
  (Class|AbilityManagerComponent|PerformAbilityOfClass (Class|PlayerStateBase|GetLocalAbilityManager) (Class|StateBase|GetSelectedAbility)))

(event EventEndState
  (bind _returnvalue (Class|StateBase|GetStateManagerComponent))
  (|CallParentFunction)
  (Class|StateManagerComponent|TryPerformStateOfClass _returnvalue (Utilities|GetClass (Class|StateManagerComponent|GetStateOfGameplayTag _returnvalue "(TagName=\"State.Idle\")")) true))

(event EventPrepareStateValues
  (|CallParentFunction)
  (Variables|/Script/Engine.CharacterMovementComponent|SetMaxWalkSpeed (Variables|/Script/Engine.Character|GetCharacterMovement (Class|PlayerStateBase|GetOwnerCharacter)) 2e+02))

(event EventTickState
  (params (TickTime :type Float%20%28single-precision%29))
  (bind _returnvalue (Class|PlayerStateBase|GetLocalAbilityManager))
  (bind _returnvalue_2 (Class|PlayerStateBase|GetLocalAbilityManager))
  (bind _returnvalue_3 (Class|AbilityManagerComponent|GetCurrentActiveAbility _returnvalue))
  (bind _abilitygameplaytag (Variables|/Script/Outline.AbilityBase|GetAbilityGameplayTag _returnvalue_3))
  (bind _returnvalue_4 (== _abilitygameplaytag "(TagName=\"Ability.Block.Start\")"))
  (if (or _returnvalue_4 (== _abilitygameplaytag "(TagName=\"Ability.Block.Loop\")"))
    (if (not (CallFunction|InputStillClicked))
      (if _returnvalue_4
        (Class|StateBase|EndState :!label _label)
        (else
          (bind _returnvalue_5 (Class|AbilityManagerComponent|TryPerformAbilityOfClass _returnvalue_2 (Utilities|GetClass (Class|AbilityManagerComponent|GetAbilityOfGameplayTag _returnvalue_2 "(TagName=\"Ability.Block.End\")")) true))
          (if (not _returnvalue_5)
            (goto _label)))))))

(fn InputStillClicked
  (return (Game|Player|IsInputKeyDown (Variables|Default|GetOwner%20Player%20Controller) (.key (Utilities|Array|Get(acopy) (Class|InputSettings|GetActionMappingbyName (Class|InputSettings|GetInputSettings) "Block"))))))

(fn CanPerformState
  (bind _returnvalue (Class|StateBase|CheckAbilitiestoRun (Utilities|Array|MakeArray (Utilities|Array|Get(acopy) (Variables|Default|GetBlock%20Abilities)))))
  (return _returnvalue))