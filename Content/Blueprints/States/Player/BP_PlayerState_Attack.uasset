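; Player attack state that builds, starts and gates the player's attack abilities through the local ability manager.
; Entering the state tries the selected ability, while exiting requests the Idle state and cancels Light Attack.
; A buffered Attack input listed in the equipped weapon's data asset restarts an active Light Attack when it can perform, then clears the buffer.
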(event EventConstructState
  (bind _returnvalue (Class|PlayerStateBase|GetLocalAbilityManager))
  ;[1 1 1] Base Functions
  (|CallParentFunction)
  (Utilities|IsValid _returnvalue
    (:Is%20Valid
      (for _array_element (Variables|Default|GetAttack%20Abilities)
        (Class|AbilityManagerComponent|ConstructAbilityOfClass _returnvalue _array_element)))))

(event EventEndState
  (bind _returnvalue (Class|PlayerStateBase|GetLocalAbilityManager))
  (bind _returnvalue_2 (Class|StateBase|GetStateManagerComponent))
  ;[1 1 1] Base Functions
  (|CallParentFunction)
  (Class|StateManagerComponent|TryPerformStateOfClass _returnvalue_2 (Utilities|GetClass (Class|StateManagerComponent|GetStateOfGameplayTag _returnvalue_2 "(TagName=\"State.Idle\")")) true)
  (Utilities|IsValid _returnvalue
    (:Is%20Valid
      (Class|AbilityBase|CancelAbility (Class|AbilityManagerComponent|GetAbilityOfGameplayTag _returnvalue "(TagName=\"Ability.Attack.LightAttack\")")))))

(event EventStartState
  (bind _returnvalue (Class|PlayerStateBase|GetLocalAbilityManager))
  ;[1 1 1] Base Functions
  (|CallParentFunction)
  (Utilities|IsValid _returnvalue
    (:Is%20Valid
      (Class|AbilityManagerComponent|TryPerformAbilityOfClass _returnvalue (Class|StateBase|GetSelectedAbility) true))))

(event EventFireBufferedInput
  (bind _returnvalue (Class|PlayerStateBase|GetBufferedInput))
  (bind _returnvalue_2 (Class|PlayerStateBase|GetLocalAbilityManager))
  (bind _returnvalue_3 (Class|AbilityManagerComponent|GetCurrentActiveAbility _returnvalue_2))
  ;[1 1 1] Comsume Buffer Input
  (bind _asbp_player_weapon_base (Utilities|Casting|CastToBP_PlayerWeaponBase (Class|CombatComponent|GetEquippedWeapon (Actor|GetComponentbyClass (Class|PlayerStateBase|GetOwnerCharacter) "/Script/Outline.PlayerCombatComponent"))))
  (if (Utilities|Array|ContainsItem (Variables|/Script/Outline.BasePlayer_PDA|GetPlayerInputs (Variables|/Script/Outline.PlayerWeaponBase|GetAssociatedDataAsset _asbp_player_weapon_base)) _returnvalue)
    (Class|PlayerInputs|SetLastFireInput(Message) (Pawn|GetController (Class|PlayerStateBase|GetOwnerCharacter)) _returnvalue)
    (switch name _returnvalue
      (:Attack
        (|SwitchGameplayTag (Variables|/Script/Outline.AbilityBase|GetAbilityGameplayTag _returnvalue_3)
          (:Ability.Attack.LightAttack
            (if (Class|AbilityBase|CanPerformAbility _returnvalue_3)
              (Class|AbilityBase|StartAbility _returnvalue_3))
            (Class|PlayerStateBase|SetBufferedInput "None")
            (Class|PlayerStateBase|RemoveAllNoneBufferingObjects)))))))

(fn CanPerformState
  (bind _returnvalue (Class|StateBase|CheckAbilitiestoRun (Variables|Default|GetAttack%20Abilities)))
  (return _returnvalue))