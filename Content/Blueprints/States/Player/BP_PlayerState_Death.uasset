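; BP_PlayerState_Death is the player's death state, which can be entered when the owner character's current health is at or below zero.
; Entry also requires that the death abilities pass the check for abilities to run.
; On start it calls the parent start, then asks the local ability manager to perform the selected ability's class with condition checking on.
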(event EventStartState
  (|CallParentFunction)
  (Class|AbilityManagerComponent|TryPerformAbilityOfClass (Class|PlayerStateBase|GetLocalAbilityManager) (Class|StateBase|GetSelectedAbility) true))

(fn CanPerformState
  (bind _returnvalue (Class|StateBase|CheckAbilitiestoRun (Variables|Default|GetDeath%20Abilities)))
  (return (and _returnvalue (<= (Class|CharacterBase|GetCurrHealth (Class|PlayerStateBase|GetOwnerCharacter)) 0.0))))