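; Player walk state for the state manager, valid while the character is not falling and has nonzero velocity.
; On start it builds the default allowed inputs for movement, combat and actions, and sets the walk speed.
; Each tick it rotates toward the targeted actor, then tries the Falling, Walk and Sprint states by gameplay tag with condition checks, stopping at the first success.
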(event EventTickState
  (params (TickTime :type Float%20%28single-precision%29))
  (bind _returnvalue (Class|StateBase|GetStateManagerComponent))
  (bind _returnvalue_2 (Class|StateBase|GetStateManagerComponent))
  (bind _returnvalue_3 (Class|StateBase|GetStateManagerComponent))
  (|CallParentFunction TickTime)
  (Class|PlayerStateBase|RotatetoTargetedActor 0.1)
  (bind _returnvalue_4 (Class|StateManagerComponent|TryPerformStateOfClass _returnvalue_3 (Utilities|GetClass (Class|StateManagerComponent|GetStateOfGameplayTag _returnvalue_3 "(TagName=\"State.Falling\")")) true))
  (if (not _returnvalue_4)
    (bind _returnvalue_5 (Class|StateManagerComponent|TryPerformStateOfClass _returnvalue_2 (Utilities|GetClass (Class|StateManagerComponent|GetStateOfGameplayTag _returnvalue_2 "(TagName=\"State.Walk\")")) true))
    (if (not _returnvalue_5)
      (Class|StateManagerComponent|TryPerformStateOfClass _returnvalue (Utilities|GetClass (Class|StateManagerComponent|GetStateOfGameplayTag _returnvalue "(TagName=\"State.Sprint\")")) true))))

(event EventStartState
  (|CallParentFunction)
  (Class|PlayerStateBase|ConstructDefaultAllowedInputs (Utilities|Array|MakeArray "Attack" "RightMouse" "Jump" "MoveForward" "MoveRight" "Evade" "Sprint" "SpecialAttack" "Equip" "Block"))
  (Variables|/Script/Engine.CharacterMovementComponent|SetMaxWalkSpeed (Variables|/Script/Engine.Character|GetCharacterMovement (Class|PlayerStateBase|GetOwnerCharacter)) 6e+02))

(fn CanPerformState
  (bind _returnvalue (Class|PlayerStateBase|GetOwnerCharacter))
  (return (and (not (AI|Components|NavMovement|IsFalling (Variables|/Script/Engine.Character|GetCharacterMovement _returnvalue))) (> (Math|Vector|VectorLength (Transformation|GetVelocity _returnvalue)) 0.0))))