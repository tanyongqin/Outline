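; Player idle state for a state-manager-driven character, which can only be entered when the owner's velocity is exactly zero.
; On start it builds the default allowed-input list, covering movement, combat, evade, sprint, jump and equip actions.
; Each tick it asks the state manager to switch, with condition checks, to the Falling state first, then to Walk if that fails, finding both by gameplay tag.
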(event EventTickState
  (params (TickTime :type Float%20%28single-precision%29))
  (bind _returnvalue (Class|StateBase|GetStateManagerComponent))
  (bind _returnvalue_2 (Class|StateBase|GetStateManagerComponent))
  (|CallParentFunction TickTime)
  (bind _returnvalue_3 (Class|StateManagerComponent|TryPerformStateOfClass _returnvalue_2 (Utilities|GetClass (Class|StateManagerComponent|GetStateOfGameplayTag _returnvalue_2 "(TagName=\"State.Falling\")")) true))
  (if (not _returnvalue_3)
    (Class|StateManagerComponent|TryPerformStateOfClass _returnvalue (Utilities|GetClass (Class|StateManagerComponent|GetStateOfGameplayTag _returnvalue "(TagName=\"State.Walk\")")) true)))

(event EventStartState
  (|CallParentFunction)
  (Class|PlayerStateBase|ConstructDefaultAllowedInputs (Utilities|Array|MakeArray "Attack" "RightMouse" "Jump" "MoveForward" "MoveRight" "Evade" "Sprint" "SpecialAttack" "Equip" "Block")))

(fn CanPerformState
  (return (== (Math|Vector|VectorLength (Transformation|GetVelocity (Class|PlayerStateBase|GetOwnerCharacter))) 0.0)))