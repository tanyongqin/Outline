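; Player hit state that runs a hit-reaction ability and returns the player to Idle when it ends.
; It can start only when a valid active state exists, that state is not Death, and the HitAbilities check passes.
; On start it performs the selected ability through the local ability manager; its attack-cancel hook is called first but is empty.
; On end it asks the state manager to switch to the Idle-tagged state.
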(event EventStartState
  (|CallParentFunction)
  (CallFunction|CancelAttackAbilities)
  (Class|AbilityManagerComponent|TryPerformAbilityOfClass (Class|PlayerStateBase|GetLocalAbilityManager) (Class|StateBase|GetSelectedAbility) true))

(event EventEndState
  (bind _returnvalue (Class|StateBase|GetStateManagerComponent))
  (|CallParentFunction)
  (Class|StateManagerComponent|TryPerformStateOfClass _returnvalue (Utilities|GetClass (Class|StateManagerComponent|GetStateOfGameplayTag _returnvalue "(TagName=\"State.Idle\")")) true))

(fn CanPerformState
  (bind _returnvalue (Class|StateBase|GetStateManagerComponent))
  (bind _returnvalue_2 (Class|StateManagerComponent|GetCurrentActiveState _returnvalue))
  (Utilities|IsValid _returnvalue_2
    (:Is%20Valid
      (if (!= (Variables|/Script/Outline.StateBase|GetStateGameplayTag _returnvalue_2) "(TagName=\"State.Death\")")
        (bind _returnvalue_3 (Class|StateBase|CheckAbilitiestoRun (Variables|Default|GetHit%20Abilities)))
        (return _returnvalue_3)))))

(fn CancelAttackAbilities)