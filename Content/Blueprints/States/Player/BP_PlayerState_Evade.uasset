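; Player state that runs the evade action within the character's state manager.
; Entry is allowed only when the owner is not falling and the evade ability passes the runnable-abilities check.
; On start it performs the selected ability through the local ability manager.
; On end it asks the state manager to switch to the state tagged State.Idle, with condition checking enabled.
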(event EventStartState
  (|CallParentFunction)
  (Class|AbilityManagerComponent|PerformAbilityOfClass (Class|PlayerStateBase|GetLocalAbilityManager) (Class|StateBase|GetSelectedAbility)))

(event EventEndState
  (bind _returnvalue (Class|StateBase|GetStateManagerComponent))
  (|CallParentFunction)
  (Class|StateManagerComponent|TryPerformStateOfClass _returnvalue (Utilities|GetClass (Class|StateManagerComponent|GetStateOfGameplayTag _returnvalue "(TagName=\"State.Idle\")")) true))

(fn CanPerformState
  (if (not (AI|Components|NavMovement|IsFalling (Variables|/Script/Engine.Character|GetCharacterMovement (Class|PlayerStateBase|GetOwnerCharacter))))
    (bind _returnvalue (Class|StateBase|CheckAbilitiestoRun (Variables|Default|GetEvade%20Ability)))
    (return _returnvalue)))