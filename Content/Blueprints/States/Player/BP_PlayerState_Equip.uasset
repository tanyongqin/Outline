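; BP_PlayerState_Equip is the player state that runs while equipping, driven by the state manager and ability manager components.
; It can be entered only when the ability check for BP_Ability_Equip passes.
; On start it performs the selected ability through the local ability manager and sets move forward and right as the default allowed inputs.
; On end it tries to switch to the Idle state by gameplay tag, with condition checking.
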(event EventEndState
  (bind _returnvalue (Class|StateBase|GetStateManagerComponent))
  (|CallParentFunction)
  (Class|StateManagerComponent|TryPerformStateOfClass _returnvalue (Utilities|GetClass (Class|StateManagerComponent|GetStateOfGameplayTag _returnvalue "(TagName=\"State.Idle\")")) true))

(event EventStartState
  (|CallParentFunction)
  (Class|AbilityManagerComponent|PerformAbilityOfClass (Class|PlayerStateBase|GetLocalAbilityManager) (Class|StateBase|GetSelectedAbility))
  (Class|PlayerStateBase|ConstructDefaultAllowedInputs (Utilities|Array|MakeArray "MoveForward" "MoveRight")))

(fn CanPerformState
  (bind _returnvalue (Class|StateBase|CheckAbilitiestoRun (Utilities|Array|MakeArray "/Game/Blueprints/Abilities/Player/BP_Ability_Equip.BP_Ability_Equip_C")))
  (return _returnvalue))