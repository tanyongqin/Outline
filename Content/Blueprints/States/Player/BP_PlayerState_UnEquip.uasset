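; Player state that handles unequipping within a state manager and ability manager setup.
; It can start only when CheckAbilitiesToRun passes for the UnEquip ability, printing a debug string when it does.
; On start it runs the parent logic and performs the selected ability through the local ability manager.
; On end it asks the state manager to switch to the Idle-tagged state, with condition checks.
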(event EventStartState
  (|CallParentFunction)
  (Class|AbilityManagerComponent|PerformAbilityOfClass (Class|PlayerStateBase|GetLocalAbilityManager) (Class|StateBase|GetSelectedAbility)))

(event EventEndState
  (bind _returnvalue (Class|StateBase|GetStateManagerComponent))
  (Class|StateManagerComponent|TryPerformStateOfClass _returnvalue (Utilities|GetClass (Class|StateManagerComponent|GetStateOfGameplayTag _returnvalue "(TagName=\"State.Idle\")")) true))

(fn CanPerformState
  (bind _returnvalue (Class|StateBase|CheckAbilitiestoRun (Utilities|Array|MakeArray (Variables|Default|GetUnEquip%20Ability))))
  (if _returnvalue
    (Development|PrintString 0 "UnEquip State Can Perform")
    (return _returnvalue)))