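; BP_PlayerState_BlockHit is the player state for taking a hit while blocking.
; It can be entered only from the NormalBlock state, and only when CheckAbilitiesToRun passes for the BlockHitAbilities.
; On start it asks the local ability manager to perform the selected ability, with condition checks.
; On end it asks the state manager to switch to the Idle state, looked up by gameplay tag.
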(event EventStartState
  (|CallParentFunction)
  (Class|AbilityManagerComponent|TryPerformAbilityOfClass (Class|PlayerStateBase|GetLocalAbilityManager) (Class|StateBase|GetSelectedAbility) true))

(event EventEndState
  (bind _returnvalue (Class|StateBase|GetStateManagerComponent))
  (|CallParentFunction)
  (Class|StateManagerComponent|TryPerformStateOfClass _returnvalue (Utilities|GetClass (Class|StateManagerComponent|GetStateOfGameplayTag _returnvalue "(TagName=\"State.Idle\")")) true))

(fn CanPerformState
  (bind _returnvalue (Class|StateBase|CheckAbilitiestoRun (Variables|Default|GetBlock%20Hit%20Abilities)))
  (return (and _returnvalue (== (Variables|/Script/Outline.StateBase|GetStateGameplayTag (Class|StateManagerComponent|GetCurrentActiveState (Class|StateBase|GetStateManagerComponent))) "(TagName=\"State.Normal Block\")"))))