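; Player sprint state for a state-manager-driven character, raising or setting movement to a sprint speed.
; It can only be entered from the Walk state while the character is not falling.
; On start it defines the allowed inputs and applies SprintSpeed to MaxWalkSpeed.
; Each tick it attempts condition-checked transitions to Idle, Falling, then Walk, resolving states by gameplay tag and stopping at the first success.
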(event EventTickState
  (params (TickTime :type Float%20%28single-precision%29))
  (bind _returnvalue (Class|StateBase|GetStateManagerComponent))
  (bind _returnvalue_2 (Class|StateBase|GetStateManagerComponent))
  (bind _returnvalue_3 (Class|StateBase|GetStateManagerComponent))
  (|CallParentFunction TickTime)
  (bind _returnvalue_4 (Class|StateManagerComponent|TryPerformStateOfClass _returnvalue_3 (Utilities|GetClass (Class|StateManagerComponent|GetStateOfGameplayTag _returnvalue_3 "(TagName=\"State.Idle\")")) true))
  (if (not _returnvalue_4)
    (bind _returnvalue_5 (Class|StateManagerComponent|TryPerformStateOfClass _returnvalue_2 (Utilities|GetClass (Class|StateManagerComponent|GetStateOfGameplayTag _returnvalue_2 "(TagName=\"State.Falling\")")) true))
    (if (not _returnvalue_5)
      (Class|StateManagerComponent|TryPerformStateOfClass _returnvalue (Utilities|GetClass (Class|StateManagerComponent|GetStateOfGameplayTag _returnvalue "(TagName=\"State.Walk\")")) true))))

(event EventStartState
  (|CallParentFunction)
  (Class|PlayerStateBase|ConstructDefaultAllowedInputs (Utilities|Array|MakeArray "Attack" "RightMouse" "Jump" "MoveForward" "MoveRight" "Dodge" "Sprint" "SpecialAttack" "Equip" "Heal"))
  (Variables|/Script/Engine.CharacterMovementComponent|SetMaxWalkSpeed (Variables|/Script/Engine.Character|GetCharacterMovement (Class|PlayerStateBase|GetOwnerCharacter)) (Variables|Default|GetSprint%20Speed)))

(fn CanPerformState
  (return (and (== (Variables|/Script/Outline.StateBase|GetStateGameplayTag (Class|StateManagerComponent|GetCurrentActiveState (Class|StateBase|GetStateManagerComponent))) "(TagName=\"State.Walk\")") (not (AI|Components|NavMovement|IsFalling (Variables|/Script/Engine.Character|GetCharacterMovement (Class|PlayerStateBase|GetOwnerCharacter)))))))