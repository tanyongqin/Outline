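; BP_AbilityBase is a base ability Blueprint that provides cooldown state and permission checks.
; ApplyAbilityCooldown sets the cooldown flag and starts a one-shot timer that fires CooldownReset to clear it, or clears it immediately when the duration is not positive.
; CanPerformAbility returns the on-cooldown flag as is, without negation, so it reads true during cooldown.
; The re-perform and cancel checks always return true.
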(event EventCooldownReset
  (Variables|Default|SetbAbilityOnCooldown false))

(event EventApplyAbilityCooldown
  (if (> (Variables|Default|GetCooldownDuration) 0.0)
    (Variables|Default|SetbAbilityOnCooldown true)
    (Utilities|Time|SetTimerbyEvent (delegate EventCooldownReset) (Variables|Default|GetCooldownDuration))
    (else
      (Variables|Default|SetbAbilityOnCooldown false))))

(fn CanPerformAbility
  (return (CallFunction|GetIsAbilityonCooldown)))

(fn CanRePerformAbility
  (return true))

(fn CanAbilitybeCanceled
  (return true))

(fn GetIsAbilityonCooldown
  (return (Variables|Default|GetbAbilityOnCooldown)))