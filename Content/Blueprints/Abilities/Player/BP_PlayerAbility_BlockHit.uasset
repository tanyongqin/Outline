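; Player ability that plays the reaction to a blocked hit.
; It is allowed only when the calculated yaw lies within a frontal arc, block montages exist, a weapon is equipped and the player is in combat.
; On start it applies the blocked impact effect through the combat component's defense property and plays a random montage, stopping others.
; On end it returns the owner's state component to Idle.
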(event EventStartAbility
  (|CallParentFunction)
  (Class|DefenseProperties|ApplyHitEffectbyClass (Variables|/Script/Outline.CombatComponent|GetOwnerDefenseProperty (Variables|/Script/Outline.PlayerCharacterBase|GetCombatComponent (Variables|Default|GetOwner%20Character))) "/Game/Blueprints/Effects/BP_ImpactEffect_Blocked.BP_ImpactEffect_Blocked_C")
  (bind _list_of_montages (CallFunction|GetAbilityMontages (Utilities|GetClass self)))
  (Class|AbilityBase|PlayAbilityMontage (.OutItem (Utilities|Array|Random _list_of_montages)) 1.0 "MontageLength" 0.0 true "None")
  (Development|PrintString 0 "Call BlockHitAbility"))

(event EventEndAbility
  (bind _owner_state_component (Variables|Default|GetOwner%20State%20Component))
  (|CallParentFunction)
  (Class|StateManagerComponent|PerformStateOfClass _owner_state_component (Utilities|GetClass (Class|StateManagerComponent|GetStateOfGameplayTag _owner_state_component "(TagName=\"State.Idle\")"))))

(fn CanPerformAbility
  (bind _owner_character (Variables|Default|GetOwner%20Character))
  (bind _returnvalue (Actor|GetComponentbyClass _owner_character "/Script/Outline.PlayerCombatComponent"))
  (bind _returnvalue_2 (Class|GeneralBlueprintFunctionLibrary|CalculateAngle))
  (if (Math|Float|InRange(Float) (.yaw _returnvalue_2) -6e+01 6e+01)
    (bind _list_of_montages (CallFunction|GetAbilityMontages (Utilities|GetClass self)))
    (if (Math|Boolean|ANDBoolean (> (Utilities|Array|Length _list_of_montages) 0) (Utilities|IsValid (Class|CombatComponent|GetEquippedWeapon _returnvalue)) (GameplayTags|HasTag (Class|CombatComponent|GetCombatStatus _returnvalue) "(TagName=\"Status.Combat.InCombat\")"))
      (return (Math|Boolean|ANDBoolean (> (Utilities|Array|Length _list_of_montages) 0) (Utilities|IsValid (Class|CombatComponent|GetEquippedWeapon _returnvalue)) (GameplayTags|HasTag (Class|CombatComponent|GetCombatStatus _returnvalue) "(TagName=\"Status.Combat.InCombat\")")))
      (else
        (Development|PrintString 0 "Can Not  Block Hit Ability")))))