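; Player evade ability that plays a directional dodge montage, available only while in combat with a weapon equipped and montages assigned.
; On start, it measures the yaw between movement input direction and actor facing, treating no input as forward.
; That angle is bucketed into four quadrants to index the ability's montage list.
; Ending the ability stops the montage and returns the owner to the Idle state.
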(event EventStartAbility
  (|CallParentFunction)
  (bind _list_of_montages (CallFunction|GetAbilityMontages (Utilities|GetClass self)))
  (bind _return_value (CallFunction|DetermineMontagebyAngle))
  (Class|AbilityBase|PlayAbilityMontage (Utilities|Array|Get(acopy) _list_of_montages _return_value) 1.0 "MontageLength" 0.0 true "None"))

(event EventEndAbility
  (bind _owner_state_component (Variables|Default|GetOwner%20State%20Component))
  (|CallParentFunction)
  (Animation|StopAnimMontage (Variables|Default|GetOwner%20Character) 0)
  (Class|StateManagerComponent|PerformStateOfClass _owner_state_component (Utilities|GetClass (Class|StateManagerComponent|GetStateOfGameplayTag _owner_state_component "(TagName=\"State.Idle\")"))))

(fn CanPerformAbility
  (bind _owner_character (Variables|Default|GetOwner%20Character))
  (bind _returnvalue (Actor|GetComponentbyClass _owner_character "/Script/Outline.PlayerCombatComponent"))
  (bind _list_of_montages (CallFunction|GetAbilityMontages (Utilities|GetClass self)))
  (return (Math|Boolean|ANDBoolean (> (Utilities|Array|Length _list_of_montages) 0) (Utilities|IsValid (Class|CombatComponent|GetEquippedWeapon _returnvalue)) (GameplayTags|HasTag (Class|CombatComponent|GetCombatStatus _returnvalue) "(TagName=\"Status.Combat.InCombat\")"))))

(fn CalcEvadeAngle
  (bind _returnvalue (Class|PlayerInputs|GetDirectionfromMovementInputs(Message) (Pawn|GetController (Variables|Default|GetOwner%20Character))))
  (if (Utilities|Operators|NotEqual(!=) :A _returnvalue)
    (return (.yaw (Math|Rotator|Delta(Rotator) (Math|Conversions|RotationFromXVector _returnvalue) (Transformation|GetActorRotation (Variables|Default|GetOwner%20Character)))))
    (else
      (return 0.0))))

(fn DetermineMontagebyAngle
  (bind _return_value (CallFunction|CalcEvadeAngle))
  (bind _output_get (LocalVariables|SetAngle _return_value))
  (if (Math|Float|InRange(Float) _output_get -45.0 45.0)
    (return 0)
    (elif (Math|Float|InRange(Float) (LocalVariables|GetAngle) 45.0 135.0)
      (return 1)
      (elif (Math|Float|InRange(Float) (LocalVariables|GetAngle) -135.0 -45.0)
        (return 2)
        (else
          (return 3))))))