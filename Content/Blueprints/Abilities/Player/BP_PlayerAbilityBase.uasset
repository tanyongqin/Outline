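; Base Blueprint for player abilities, providing shared owner setup and a montage lookup.
; On construction it requires a valid ability gameplay tag, then caches the performing player character and its controller's StateManagerComponent, printing a notice if the tag or character cast fails.
; GetAbilityMontages searches the equipped weapon's data asset for a given ability and returns its montage list, so animations are data-driven per weapon.
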(event EventConstructAbility
  (|CallParentFunction)
  (if (GameplayTags|IsGameplayTagValid (Variables|Default|GetAbilityGameplayTag))
    (bind _asbp_player_character (Utilities|Casting|CastToBP_PlayerCharacter (Class|AbilityBase|GetPerformingActor))
      (:then
        (bind _output_get (Variables|Default|SetOwner%20Character _asbp_player_character))
        (bind _asbp_player_controller (Utilities|Casting|CastToBP_PlayerController (Pawn|GetController _output_get)))
        (Variables|Default|SetOwner%20State%20Component (Actor|GetComponentbyClass _asbp_player_controller "/Script/Outline.StateManagerComponent")))
      (:CastFailed
        (Development|PrintString 0 (Utilities|String|Append "Cast Character Fail:" (Utilities|GetDisplayName self)))))
    (else
      (Development|PrintString 0 (Utilities|String|Append "Developer Notice: You Forgot To Specify Gameplay Tag For Ability " (Utilities|GetDisplayName self))))))

(fn GetAbilityMontages
  (params (Ability%20To%20Look%20For :type BP%20Player%20Ability%20Base%20Class%20Reference))
  (bind _asbp_player_weapon_base (Utilities|Casting|CastToBP_PlayerWeaponBase (Class|CombatComponent|GetEquippedWeapon (Variables|/Script/Outline.PlayerCharacterBase|GetCombatComponent (Variables|Default|GetOwner%20Character))))
    (:then
      (for _array_element (Variables|/Script/Outline.BasePlayer_PDA|GetAbilities (Variables|/Script/Outline.PlayerWeaponBase|GetAssociatedDataAsset _asbp_player_weapon_base))
        (if (== (.Ability (Utilities|Struct|BreakAbilityMontages _array_element)) Ability%20To%20Look%20For)
          (return (.ListOfMontages (Utilities|Struct|BreakAbilityMontages _array_element))))))
    (:CastFailed
      _))
  (return 0))