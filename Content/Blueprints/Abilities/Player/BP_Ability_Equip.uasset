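; Player ability that draws the equipped weapon and puts the character into combat.
; It is allowed only from Idle, Walk or Sprint, with montages available, a valid equipped weapon and no existing InCombat status.
; On start it plays a random ability montage, switches the anim instance to the in-combat moveset, sets walk speed and adds the InCombat tag.
; On end it performs the Idle state.
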(event EventStartAbility
  (bind _owner_character (Variables|Default|GetOwner%20Character))
  (|CallParentFunction)
  (bind _list_of_montages (CallFunction|GetAbilityMontages (Utilities|GetClass self)))
  (Utilities|IsValid (.OutItem (Utilities|Array|Random _list_of_montages))
    (:Is%20Valid
      (Class|AbilityBase|PlayAbilityMontage (.OutItem (Utilities|Array|Random _list_of_montages)) 1.0 "Duration" 0.0 true "None")
      (Class|GeneralInterface|AssignMoveset(Message) (Components|SkeletalMesh|GetAnimInstance (Variables|/Script/Engine.Character|GetMesh _owner_character)) "EM_IN_COMBAT")
      (Variables|/Script/Engine.CharacterMovementComponent|SetMaxWalkSpeed (Variables|/Script/Engine.Character|GetCharacterMovement _owner_character) 4.5e+02)
      (Class|CombatComponent|ModifyCombatStatus (Variables|/Script/Outline.PlayerCharacterBase|GetCombatComponent (Variables|Default|GetOwner%20Character)) "(TagName=\"Status.Combat.InCombat\")" "Add"))))

(event EventEndAbility
  (bind _owner_state_component (Variables|Default|GetOwner%20State%20Component))
  (|CallParentFunction)
  (Class|StateManagerComponent|PerformStateOfClass _owner_state_component (Utilities|GetClass (Class|StateManagerComponent|GetStateOfGameplayTag _owner_state_component "(TagName=\"State.Idle\")"))))

(fn CanPerformAbility
  (bind _owner_state_component (Variables|Default|GetOwner%20State%20Component))
  (bind _owner_character (Variables|Default|GetOwner%20Character))
  (bind _currentactivestate (Variables|/Script/Outline.StateManagerComponent|GetCurrentActiveState _owner_state_component))
  (bind _combatcomponent (Variables|/Script/Outline.PlayerCharacterBase|GetCombatComponent _owner_character))
  (bind _stategameplaytag (Variables|/Script/Outline.StateBase|GetStateGameplayTag _currentactivestate))
  (Utilities|IsValid _currentactivestate
    (:Is%20Valid
      (bind _list_of_montages (CallFunction|GetAbilityMontages (Utilities|GetClass self)))
      (return (Math|Boolean|ANDBoolean (> (Utilities|Array|Length _list_of_montages) 0) (Math|Boolean|ORBoolean (== _stategameplaytag "(TagName=\"State.Idle\")") (== _stategameplaytag "(TagName=\"State.Walk\")") (== _stategameplaytag "(TagName=\"State.Sprint\")")) (not (GameplayTags|HasTag (Class|CombatComponent|GetCombatStatus _combatcomponent) "(TagName=\"Status.Combat.InCombat\")")) (Utilities|IsValid (Class|CombatComponent|GetEquippedWeapon _combatcomponent)))))
    (:Is%20Not%20Valid
      (return false))))