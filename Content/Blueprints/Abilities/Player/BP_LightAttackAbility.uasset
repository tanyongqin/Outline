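; Player light attack ability that plays a melee combo, advancing one montage each time the ability starts.
; It requires an "Attack" input, available montages, a valid equipped weapon and an in-combat status from PlayerCombatComponent.
; A combo index selects the montage and wraps after the last.
; Cancelling resets the combo, while ending also resets it and asks the state component to return to Idle.
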(event EventCancelAbility
  (Variables|Default|SetCombo 0))

(event EventStartAbility
  (|CallParentFunction)
  (bind _list_of_montages (CallFunction|GetAbilityMontages (Utilities|GetClass self)))
  (Class|AbilityBase|PlayAbilityMontage (Utilities|Array|Get(acopy) _list_of_montages (Variables|Default|GetCombo)) 1.0 "Duration" 0.0 true "None")
  (Variables|Default|SetCombo (select (== (+ (Variables|Default|GetCombo) 1) (Utilities|Array|Length _list_of_montages)) 0 (+ (Variables|Default|GetCombo) 1))))

(event EventEndAbility
  (bind _owner_state_component (Variables|Default|GetOwner%20State%20Component))
  (|CallParentFunction)
  (Variables|Default|SetCombo 0)
  (Class|StateManagerComponent|TryPerformStateOfClass _owner_state_component (Utilities|GetClass (Class|StateManagerComponent|GetStateOfGameplayTag _owner_state_component "(TagName=\"State.Idle\")")) true))

(fn CanPerformAbility
  (bind _owner_character (Variables|Default|GetOwner%20Character))
  (bind _returnvalue (Actor|GetComponentbyClass _owner_character "/Script/Outline.PlayerCombatComponent"))
  (bind _returnvalue_2 (Class|PlayerInputs|GetLastFireInput(Message) (Pawn|GetController (Variables|Default|GetOwner%20Character))))
  (if (== _returnvalue_2 "Attack")
    (bind _list_of_montages (CallFunction|GetAbilityMontages (Utilities|GetClass self)))
    (return (Math|Boolean|ANDBoolean (> (Utilities|Array|Length _list_of_montages) 0) (Utilities|IsValid (Class|CombatComponent|GetEquippedWeapon _returnvalue)) (GameplayTags|HasTag (Class|CombatComponent|GetCombatStatus _returnvalue) "(TagName=\"Status.Combat.InCombat\")") true))
    (else
      (return false))))