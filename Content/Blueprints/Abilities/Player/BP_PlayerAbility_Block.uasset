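; Player block ability that plays a random block montage while active.
; Activation requires an available montage for the ability class, an equipped weapon on the player combat component and the InCombat gameplay tag in its combat status.
; Starting stops other montages and plays one picked at random from that class's set.
; Ending stops the montage and has the owner's state component perform the Idle state.
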(event EventStartAbility
  (|CallParentFunction)
  (bind _list_of_montages (CallFunction|GetAbilityMontages (Utilities|GetClass self)))
  (Class|AbilityBase|PlayAbilityMontage (.OutItem (Utilities|Array|Random _list_of_montages)) 1.0 "MontageLength" 0.0 true "None"))

(event EventEndAbility
  (bind _owner_state_component (Variables|Default|GetOwner%20State%20Component))
  (|CallParentFunction)
  (Animation|StopAnimMontage (Variables|Default|GetOwner%20Character) 0)
  (Class|StateManagerComponent|PerformStateOfClass _owner_state_component (Utilities|GetClass (Class|StateManagerComponent|GetStateOfGameplayTag _owner_state_component "(TagName=\"State.Idle\")"))))

(fn CanPerformAbility
  (bind _owner_character (Variables|Default|GetOwner%20Character))
  (bind _returnvalue (Actor|GetComponentbyClass _owner_character "/Script/Outline.PlayerCombatComponent"))
  (bind _list_of_montages (CallFunction|GetAbilityMontages (Utilities|GetClass self)))
  (return (Math|Boolean|ANDBoolean (> (Utilities|Array|Length _list_of_montages) 0) (Utilities|IsValid (Class|CombatComponent|GetEquippedWeapon _returnvalue)) (GameplayTags|HasTag (Class|CombatComponent|GetCombatStatus _returnvalue) "(TagName=\"Status.Combat.InCombat\")"))))