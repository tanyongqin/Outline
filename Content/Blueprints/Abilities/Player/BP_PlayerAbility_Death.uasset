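; Player death ability that plays a death montage when it starts.
; StartAbility runs the parent logic, then plays the first montage looked up by the ability's own class, stopping all other montages.
; CanPerformAbility allows the ability only when that class lookup returns at least one montage.
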(event EventStartAbility
  (|CallParentFunction)
  (bind _list_of_montages (CallFunction|GetAbilityMontages (Utilities|GetClass self)))
  (Class|AbilityBase|PlayAbilityMontage (Utilities|Array|Get(acopy) _list_of_montages) 1.0 "MontageLength" 0.0 true "None"))

(fn CanPerformAbility
  (bind _list_of_montages (CallFunction|GetAbilityMontages (Utilities|GetClass self)))
  (return (> (Utilities|Array|Length _list_of_montages) 0)))