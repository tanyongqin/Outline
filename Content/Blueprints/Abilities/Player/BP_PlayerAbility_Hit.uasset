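; Player hit-reaction ability that plays a directional montage when the character is struck.
; It can run only with montages available, a weapon equipped and the InCombat status tag present.
; On start, the yaw angle to the owner of the received attack selects the first montage within ±90 degrees, otherwise the second, stopping other montages.
; On end, it returns the state component to Idle.
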(event EventStartAbility
  (|CallParentFunction)
  (bind _list_of_montages (CallFunction|GetAbilityMontages (Utilities|GetClass self)))
  (Variables|Default|SetHit%20Reaction%20Montages _list_of_montages)
  (bind _output_get (Variables|Default|SetReceived%20Attack%20Property (Variables|/Script/Outline.CombatComponent|GetReceivedAttackProperty (Actor|GetComponentbyClass (Variables|Default|GetOwner%20Character) "/Script/Outline.PlayerCombatComponent"))))
  (bind _returnvalue (Class|GeneralBlueprintFunctionLibrary|CalculateAngle (Variables|Default|GetOwner%20Character) (Class|AttackProperties|GetAttackPropertyOwner _output_get)))
  (if (Math|Float|InRange(Float) (.yaw _returnvalue) -9e+01 9e+01)
    (Variables|Default|SetMontage%20Index 0)
    (else
      (Variables|Default|SetMontage%20Index 1)))
  (Class|AbilityBase|PlayAbilityMontage (Utilities|Array|Get(acopy) (Variables|Default|GetHit%20Reaction%20Montages) (Variables|Default|GetMontage%20Index)) 1.0 "MontageLength" 0.0 true "None"))

(event EventEndAbility
  (bind _owner_state_component (Variables|Default|GetOwner%20State%20Component))
  (|CallParentFunction)
  (Class|StateManagerComponent|PerformStateOfClass _owner_state_component (Utilities|GetClass (Class|StateManagerComponent|GetStateOfGameplayTag _owner_state_component "(TagName=\"State.Idle\")"))))

(fn CanPerformAbility
  (bind _owner_character (Variables|Default|GetOwner%20Character))
  (bind _returnvalue (Actor|GetComponentbyClass _owner_character "/Script/Outline.PlayerCombatComponent"))
  (Utilities|IsValid (Class|AbilityBase|GetPerformingActor)
    (:Is%20Valid
      (bind _list_of_montages (CallFunction|GetAbilityMontages (Utilities|GetClass self)))
      (return (Math|Boolean|ANDBoolean (> (Utilities|Array|Length _list_of_montages) 0) (Utilities|IsValid (Class|CombatComponent|GetEquippedWeapon _returnvalue)) (GameplayTags|HasTag (Class|CombatComponent|GetCombatStatus _returnvalue) "(TagName=\"Status.Combat.InCombat\")"))))
    (:Is%20Not%20Valid
      (Development|PrintString 0 "OwnerCharacter IS NONE"))))