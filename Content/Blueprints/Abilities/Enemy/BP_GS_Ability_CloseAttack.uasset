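; Enemy close-range melee attack ability that plays one of two montages chosen at random.
; StartAbility calls the parent, picks montage index 0 or 1 from the class's ability montage list and plays it, stopping other montages.
; CanPerformAbility allows the attack only when the calculated distance is within a short range and at least one montage exists.
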(event EventStartAbility
  (|CallParentFunction)
  (Variables|Default|SetCombo (Math|Integer|SelectInt 0 1 (Math|Random|RandomBool)))
  (bind _listofmontages (CallFunction|GetAbilityMontages (Utilities|GetClass self)))
  (Class|AbilityBase|PlayAbilityMontage (Utilities|Array|Get(acopy) _listofmontages (Variables|Default|GetCombo)) 1.0 "MontageLength" 0.0 true "None"))

(fn CanPerformAbility
  (bind _listofmontages (CallFunction|GetAbilityMontages (Utilities|GetClass self)))
  (bind _distance (CallFunction|CalcDistance))
  (return (and (Math|Float|InRange(Float) _distance 1.0 4e+02) (> (Utilities|Array|Length _listofmontages) 0))))