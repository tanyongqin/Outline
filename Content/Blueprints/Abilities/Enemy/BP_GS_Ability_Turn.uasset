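; Enemy turn-in-place ability that plays a turn montage to rotate the character toward its combat target.
; StartAbility caches the starting transform and plays the class's montage at MontageIndex.
; Each tick, a montage curve scales the yaw offset to the target, divided by DivisionValue, and actor rotation lerps halfway there.
; CanPerformAbility requires montages and yaw within 45–115 degrees; the negative-side check has reversed Min/Max bounds.
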(event EventStartAbility
  (bind _currentperformingactor (Class|AbilityBase|GetPerformingActor))
  (|CallParentFunction)
  (bind _listofmontages (CallFunction|GetAbilityMontages (Utilities|GetClass self)))
  (if (> (Utilities|Array|Length _listofmontages) (Variables|Default|GetMontage%20Index))
    (Variables|Default|SetTurn%20Montage (Utilities|Array|Get(acopy) _listofmontages (Variables|Default|GetMontage%20Index)))
    (Variables|Default|SetOriginal%20Location (Transformation|GetActorLocation _currentperformingactor))
    (Variables|Default|SetOriginal%20Rotation (Transformation|GetActorRotation _currentperformingactor))
    (Class|AbilityBase|PlayAbilityMontage (Variables|Default|GetTurn%20Montage) 1.0 "MontageLength" 0.0 true "None")
    (bind _asenemy_character_base (Utilities|Casting|CastToEnemyCharacterBase (Class|AbilityBase|GetPerformingActor)))
    (Variables|Default|SetOwner%20Character _asenemy_character_base)))

(event EventTickAbility
  (params (TickTime :type Float%20%28single-precision%29))
  (bind _curve_name (Variables|Default|GetCurve%20Name))
  (bind _original_rotation (Variables|Default|GetOriginal%20Rotation))
  (bind _owner_character (Variables|Default|GetOwner%20Character))
  (bind (_roll _pitch _yaw) (Math|Rotator|BreakRotator _original_rotation))
  (bind _mesh (Variables|/Script/Engine.Character|GetMesh _owner_character))
  (bind _returnvalue (Components|SkeletalMesh|GetAnimInstance _mesh))
  (bind _returnvalue_2 (Animation|Curves|GetCurveValue _returnvalue _curve_name))
  (bind _returnvalue_3 (Class|EnemyCombatComponent|GetCombatTarget (Variables|/Script/Outline.EnemyCharacterBase|GetCombatComponent (Variables|Default|GetOwner%20Character))))
  (Variables|Default|SetCombat%20Target _returnvalue_3)
  (if (Math|Boolean|ANDBoolean (Utilities|Operators|NotEqual(!=) :A (Variables|Default|GetOriginal%20Location)) (Animation|Montage|MontageIsPlaying _returnvalue (Class|AbilityBase|GetActiveAbilityMontage)) (> _returnvalue_2 0.0))
    (Transformation|SetActorRotation (Variables|Default|GetOwner%20Character) (Math|Rotator|Lerp(Rotator) (Transformation|GetActorRotation (Variables|Default|GetOwner%20Character)) (Math|Rotator|MakeRotator _roll _pitch (+ _yaw (* _returnvalue_2 (/ (.yaw (Math|Rotator|Delta(Rotator) (Variables|Default|GetOriginal%20Rotation) (Math|Rotator|FindLookatRotation (Variables|Default|GetOriginal%20Location) (Transformation|GetActorLocation (Variables|Default|GetCombat%20Target))))) (Variables|Initialization|GetDivision%20Value))))) 0.5) true)))

(fn CanPerformAbility
  (bind _listofmontages (CallFunction|GetAbilityMontages (Utilities|GetClass self)))
  (bind _return_value (CallFunction|CalcPitchandYaw))
  (return (and (or (Math|Float|InRange(Float) (.yaw _return_value) 45.0 115.0) (Math|Float|InRange(Float) (.yaw _return_value) -45.0 -115.0)) (> (Utilities|Array|Length _listofmontages) 0))))