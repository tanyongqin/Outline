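; Enemy roll ability that plays one of two directional montages based on the calculated yaw.
; It can run only when montages exist, the calculated distance is short and the yaw lies within the front half-circle.
; On start, negative yaw picks the first montage and positive yaw the second.
; The montage starts partway in, at a time offset, and stops all other montages.
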(event EventStartAbility
  (|CallParentFunction)
  (bind _listofmontages (CallFunction|GetAbilityMontages (Utilities|GetClass self)))
  (Class|AbilityBase|PlayAbilityMontage (Utilities|Array|Get(acopy) _listofmontages (CallFunction|DetermineMontageIndex)) 1.0 "Duration" 1.0 true "None"))

(fn CanPerformAbility
  (bind _listofmontages (CallFunction|GetAbilityMontages (Utilities|GetClass self)))
  (bind _distance (CallFunction|CalcDistance))
  (bind _return_value (CallFunction|CalcPitchandYaw))
  (return (Math|Boolean|ANDBoolean (Math|Float|InRange(Float) _distance 0.0 1e+02) (> (Utilities|Array|Length _listofmontages) 0) (Math|Float|InRange(Float) (.yaw _return_value) -9e+01 9e+01))))

(fn DetermineMontageIndex
  (bind _return_value (CallFunction|CalcPitchandYaw))
  (if (Math|Float|InRange(Float) (.yaw _return_value) -9e+01 0.0)
    (return 0)
    (else
      (return 1))))