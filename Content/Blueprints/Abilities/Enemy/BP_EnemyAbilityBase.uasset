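; Base Blueprint for enemy abilities, providing montage lookup and helper queries on the performing enemy's combat target.
; Montages come from the enemy character's data asset by matching the requested ability in its Abilities list.
; Distance and pitch/yaw helpers read the target from EnemyCombatComponent and return zero without a valid one.
; The angles are the actor's rotation relative to the look-at rotation toward that target, with roll zeroed.
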(fn GetAbilityMontages
  (params (AbilityToFind :type BP%20Enemy%20Ability%20Base%20Class%20Reference))
  (bind _asenemy_character_base (Utilities|Casting|CastToEnemyCharacterBase (Class|AbilityBase|GetPerformingActor)))
  (Utilities|IsValid _asenemy_character_base
    (:Is%20Valid
      (Utilities|IsValid (Variables|/Script/Outline.EnemyCharacterBase|GetAssociatedDataAsset _asenemy_character_base)
        (:Is%20Valid
          (for _array_element (Variables|/Script/Outline.BaseEnemy_PDA|GetAbilities (Variables|/Script/Outline.EnemyCharacterBase|GetAssociatedDataAsset _asenemy_character_base))
            (if (== (.Ability (Utilities|Struct|BreakAbilityMontages _array_element)) AbilityToFind)
              (return (.ListOfMontages (Utilities|Struct|BreakAbilityMontages _array_element))))))))))

(fn CalcDistance
  (bind _currentperformingactor (Class|AbilityBase|GetPerformingActor))
  (bind _returnvalue (Class|EnemyCombatComponent|GetCombatTarget (Actor|GetComponentbyClass _currentperformingactor "/Script/Outline.EnemyCombatComponent")))
  (Utilities|IsValid _returnvalue
    (:Is%20Valid
      (return (Math|Vector|VectorLength (- (Transformation|GetActorLocation _returnvalue) (Transformation|GetActorLocation _currentperformingactor)))))
    (:Is%20Not%20Valid
      (return 0.0))))

(fn CalcPitchandYaw
  (bind _currentperformingactor (Class|AbilityBase|GetPerformingActor))
  (bind _returnvalue (Class|EnemyCombatComponent|GetCombatTarget (Actor|GetComponentbyClass _currentperformingactor "/Script/Outline.EnemyCombatComponent")))
  (Utilities|IsValid _returnvalue
    (:Is%20Valid
      (return (Math|Rotator|MakeRotator 0.0 (.pitch (Math|Rotator|Delta(Rotator) (Transformation|GetActorRotation _currentperformingactor) (Math|Rotator|FindLookatRotation (Transformation|GetActorLocation _currentperformingactor) (Transformation|GetActorLocation _returnvalue)))) (.yaw (Math|Rotator|Delta(Rotator) (Transformation|GetActorRotation _currentperformingactor) (Math|Rotator|FindLookatRotation (Transformation|GetActorLocation _currentperformingactor) (Transformation|GetActorLocation _returnvalue)))))))
    (:Is%20Not%20Valid
      (return "0, 0, 0"))))