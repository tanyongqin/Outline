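; Enemy death ability that plays a randomly chosen death montage when it starts.
; On start it calls the parent logic, then picks from the montages looked up for its own class and plays one, stopping all other montages.
; The ability can only be performed when at least one montage exists for that class.
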(event EventStartAbility
  (|CallParentFunction)
  (bind _listofmontages (CallFunction|GetAbilityMontages (Utilities|GetClass self)))
  (Class|AbilityBase|PlayAbilityMontage (.OutItem (Utilities|Array|Random _listofmontages)) 1.0 "MontageLength" 0.0 true "None"))

(fn CanPerformAbility
  (bind _listofmontages (CallFunction|GetAbilityMontages (Utilities|GetClass self)))
  (return (> (Utilities|Array|Length _listofmontages) 0)))