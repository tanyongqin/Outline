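; Enemy jump attack ability that leaps the performing actor toward its combat target's position.
; On start it plays the first ability montage and caches the owner and target locations, so the leap does not track the target.
; Each tick an animation curve scales the horizontal offset between them, moving the actor without sweep at its starting height.
; It is usable only with a montage available and within set distance and yaw ranges.
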(event EventStartAbility
  (bind _listofmontages (CallFunction|GetAbilityMontages (Utilities|GetClass self)))
  (Class|AbilityBase|PlayAbilityMontage (Utilities|Array|Get(acopy) _listofmontages) 1.0 "Duration" 0.0 true "None")
  (Variables|Default|SetOwner%20Location (Transformation|GetActorLocation (Class|AbilityBase|GetPerformingActor)))
  (bind _returnvalue (Class|EnemyCombatComponent|GetCombatTarget (Actor|GetComponentbyClass (Class|AbilityBase|GetPerformingActor) "/Script/Outline.EnemyCombatComponent")))
  (Variables|Default|SetTarget%20Location (Transformation|GetActorLocation _returnvalue)))

(event EventTickAbility
  (params (TickTime :type Float%20%28single-precision%29))
  (bind _target_location (Variables|Default|GetTarget%20Location))
  (bind _owner_location (Variables|Default|GetOwner%20Location))
  (bind _returnvalue (- _target_location _owner_location))
  (bind _ascharacter (Utilities|Casting|CastToCharacter (Class|AbilityBase|GetPerformingActor)))
  (Transformation|SetActorLocation (Class|AbilityBase|GetPerformingActor) (+ (Variables|Default|GetOwner%20Location) (Math|Vector|MakeVector (* (.x _returnvalue) (Animation|Curves|GetCurveValue (Components|SkeletalMesh|GetAnimInstance (Variables|/Script/Engine.Character|GetMesh _ascharacter)) "XLocationOffset")) (* (.y _returnvalue) (Animation|Curves|GetCurveValue (Components|SkeletalMesh|GetAnimInstance (Variables|/Script/Engine.Character|GetMesh _ascharacter)) "XLocationOffset")) 0.0)) false false))

(fn CanPerformAbility
  (bind _listofmontages (CallFunction|GetAbilityMontages (Utilities|GetClass self)))
  (bind _distance (CallFunction|CalcDistance))
  (bind _return_value (CallFunction|CalcPitchandYaw))
  (return (Math|Boolean|ANDBoolean (Math|Float|InRange(Float) _distance 4e+02 8.5e+02 false) (> (Utilities|Array|Length _listofmontages) 0) (Math|Float|InRange(Float) (.yaw _return_value) -6e+01 6e+01))))