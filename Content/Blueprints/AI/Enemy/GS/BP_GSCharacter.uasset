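; BP_GSCharacter is an enemy AI character Blueprint that shows or hides a lock-on marker on itself.
; ToggleTargetingPoint creates a screen-space widget component at runtime, fills it with a WBP_LockOn widget and snaps it to the capsule.
; Toggling off destroys that component, and validity checks prevent duplicate markers.
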(event EventBeginPlay)

(event Collision|EventActorBeginOverlap
  (params (OtherActor :type Actor%20Object%20Reference)))

(event EventTick
  (params (DeltaSeconds :type Float%20%28single-precision%29)))

(event EventToggleTargetingPoint
  (params (bToggle :type Boolean))
  (if bToggle
    (Utilities|IsValid (Variables|Default|GetCreated%20Widget%20Component)
      (:Is%20Not%20Valid
        (bind _returnvalue (AddComponent|AddWidgetComponent false))
        (bind _output_get (Variables|Default|SetCreated%20Widget%20Component _returnvalue))
        (Class|WidgetComponent|SetWidgetSpace _output_get "Screen")
        (Class|WidgetComponent|SetDrawSize (Variables|Default|GetCreated%20Widget%20Component) "(X=30.000000,Y=30.000000)")
        (bind _returnvalue_2 (UserInterface|CreateWidget "/Game/Blueprints/AI/WBP_LockOn.WBP_LockOn_C"))
        (UserInterface|SetWidget (Variables|Default|GetCreated%20Widget%20Component) _returnvalue_2)
        (Transformation|AttachComponentToComponent (Variables|Default|GetCreated%20Widget%20Component) (Variables|Default|GetCapsuleComponent) "None" "SnapToTarget" "SnapToTarget" "SnapToTarget" true)))
    (else
      (Utilities|IsValid (Variables|Default|GetCreated%20Widget%20Component)
        (:Is%20Valid
          (Components|DestroyComponent (Variables|Default|GetCreated%20Widget%20Component)))))))

(fn ConstructionScript)