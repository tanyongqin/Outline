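; Katana weapon pickup that equips itself when the player character overlaps its sphere.
; Equipping unequips any current weapon, switches the owner to the samurai anim Blueprint and assigns a common moveset.
; It creates katana and scabbard meshes on character sockets, registers their equip sockets and binds a right-hand weapon trace to the blade.
; It then applies attributes, registers with PlayerCombatComponent and destroys the sphere; a posture modifier is left unconnected.
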(event OnComponentBeginOverlap(Sphere)
  (params (OverlappedComponent :type Primitive%20Component%20Object%20Reference) (OtherActor :type Actor%20Object%20Reference) (OtherComp :type Primitive%20Component%20Object%20Reference) (OtherBodyIndex :type Integer) (bFromSweep :type Boolean) (SweepResult :type Hit%20Result%20Structure%20%28by%20ref%29))
  (if (== OtherActor (Game|GetPlayerCharacter 0))
    (Actor|SetOwner OtherActor)
    (Class|WeaponBase|EquipWeapon)))

(event EventBeginPlay)

(event EventEquipWeapon
  (bind _returnvalue (Components|GetOwner))
  (bind _returnvalue_2 (Actor|GetComponentbyClass _returnvalue "/Script/Outline.PlayerCombatComponent"))
  (bind _returnvalue_3 (Class|CombatComponent|GetEquippedWeapon _returnvalue_2))
  (Utilities|IsValid _returnvalue
    (:Is%20Valid
      (Utilities|IsValid _returnvalue_3
        (:Is%20Valid
          (Class|WeaponBase|UnEquipWeapon _returnvalue_3))
        (:Is%20Not%20Valid
          _))
      (bind _ascharacter_base (Utilities|Casting|CastToCharacterBase (Components|GetOwner)))
      (bind _output_get (Variables|Default|SetOwnedCharacter _ascharacter_base))
      (Class|SkeletalMeshComponent|SetAnimClass (Variables|/Script/Engine.Character|GetMesh _output_get) "/Game/Blueprints/Character/SamuraiAnimBP.SamuraiAnimBP_C")
      (Class|GeneralInterface|AssignMoveset(Message) (Variables|Default|GetOwnedCharacter) "EM_COMMON")
      (Utilities|FlowControl|Sequence
        (:then_0
          (bind _createdtraceobject (Class|CollisionManagerComponent|ConstructTraceOfClass (Actor|GetComponentbyClass (Variables|Default|GetOwnedCharacter) "/Script/Outline.CollisionManagerComponent") "/Script/Outline.TraceBase"))
          (bind _output_get_2 (Variables|Default|SetKatana%20Trace _createdtraceobject))
          (Variables|/Script/Outline.TraceBase|SetTraceGameplayTag _output_get_2 "(TagName=\"Trace.Right Hand Weapon\")")
          (bind _returnvalue_4 (AddComponent|AddStaticMeshComponent false))
          (bind _output_get_3 (Variables|Default|SetKatana%20Mesh%20Component _returnvalue_4))
          (Collision|SetCollisionEnabled _output_get_3 "NoCollision")
          (Transformation|AttachComponentToComponent (Variables|Default|GetKatana%20Mesh%20Component) (Variables|/Script/Engine.Character|GetMesh (Variables|Default|GetOwnedCharacter)) "katana1" "SnapToTarget" "SnapToTarget" "SnapToTarget" true)
          (Components|StaticMesh|SetStaticMesh (Variables|Default|GetKatana%20Mesh%20Component) (Variables|Default|GetKatana%20Mesh))
          (Class|TraceBase|SetTraceMeshInfo (Variables|Default|GetKatana%20Trace) (Variables|Default|GetKatana%20Mesh%20Component) (Utilities|Array|MakeArray "Start" "End"))
          (Class|WeaponBase|RegisterWeapon (Utilities|Struct|MakeWeaponDetails (Variables|Default|GetKatana%20Mesh%20Component) "katana3" "katana1")))
        (:then_1
          (bind _returnvalue_5 (AddComponent|AddStaticMeshComponent false))
          (bind _output_get_4 (Variables|Default|SetScabbard%20Mesh%20Component _returnvalue_5))
          (Collision|SetCollisionEnabled _output_get_4 "NoCollision")
          (Transformation|AttachComponentToComponent (Variables|Default|GetScabbard%20Mesh%20Component) (Variables|/Script/Engine.Character|GetMesh (Variables|Default|GetOwnedCharacter)) "scabbard1" "SnapToTarget" "SnapToTarget" "SnapToTarget" true)
          (Components|StaticMesh|SetStaticMesh (Variables|Default|GetScabbard%20Mesh%20Component) (Variables|Default|GetScabbard%20Mesh))
          (Class|WeaponBase|RegisterWeapon (Utilities|Struct|MakeWeaponDetails (Variables|Default|GetScabbard%20Mesh%20Component) "scabbard1" "scabbard1")))
        (:then_2
          (Class|PlayerWeaponBase|SetAttributesandStates)
          (Class|CombatComponent|SetEquippedWeapon (Actor|GetComponentbyClass (Variables|Default|GetOwnedCharacter) "/Script/Outline.PlayerCombatComponent") self)
          (Components|DestroyComponent (Variables|Default|GetSphere)))))))

(fn ConstructionScript)